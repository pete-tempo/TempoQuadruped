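; Unitree Go2 pawn whose skeletal mesh is animated through a ControlRig component.
; On pre-initialize, the rig maps the complete skeletal mesh as output, and BeginPlay adds a small controller pitch input.
; Before each forward solve, the Target control moves to the actor's location.
; Target takes the actor's rotation only when its prior rig-space position is at least DeadZone from the actor's location, otherwise keeping its own.
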(event OnPreInitializeDelegate(ControlRig)
  (params (Component :type Control%20Rig%20Component%20Object%20Reference))
  (Class|ControlRigComponent|AddMappedCompleteSkeletalMesh Component (Variables|Default|GetSkeletalMesh) "Output"))

(event OnPreForwardsSolveDelegate(ControlRig)
  (params (Component :type Control%20Rig%20Component%20Object%20Reference))
  (bind _returnvalue (Transformation|GetActorTransform))
  (bind _returnvalue_2 (Class|ControlRigComponent|GetControlTransform Component "Target" "RigSpace"))
  (bind _controlrig (Variables|Default|GetControlRig))
  (if (< (Math|Vector|Distance(Vector) (.location _returnvalue_2) (.location _returnvalue)) (Variables|Default|GetDeadZone))
    (Class|ControlRigComponent|SetControlTransform _controlrig "Target" (Math|Transform|MakeTransform (.location _returnvalue) (.rotation _returnvalue_2) "1.000000,1.000000,1.000000") "RigSpace")
    (else
      (Class|ControlRigComponent|SetControlTransform _controlrig "Target" (Math|Transform|MakeTransform (.location _returnvalue) (.rotation _returnvalue) "1.000000,1.000000,1.000000") "RigSpace"))))

(event EventBeginPlay
  (Pawn|Input|AddControllerPitchInput 1e+01))

(event Collision|EventActorBeginOverlap
  (params (OtherActor :type Actor%20Object%20Reference)))

(event EventTick
  (params (DeltaSeconds :type Float%20%28single-precision%29)))

(fn ConstructionScript)